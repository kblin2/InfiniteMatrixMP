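; BP_TunnelSpawner builds a chain of BP_Tunnel segments and populates it with health packs and enemies.
; On BeginPlay it clears existing tunnels, then spawns a short starting chain from the player pawn's location, each segment attaching at the previous one's SpawnPoint.
; Each segment gets a spawner reference and randomized walls, then rolls for a health pack or, failing that, an enemy at a randomly offset position.
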(event `self.ReceiveBeginPlay`
  (`self.Spawn Intial Tunnels`))

(fn `Spawn Intial Tunnels`
  (`|ExecutionSequence`
    (:`then_0`
      (bind _outactors (`GameplayStatics.GetAllActorsOfClass` "/Game/InfiniteMatrix/Blueprints/BP_Tunnel.BP_Tunnel_C"))
      (for _array_element _outactors
        (`self.K2_DestroyActor` _array_element)))
    (:`then_1`
      (for _ (range 3)
        (`/Engine/EditorBlueprintResources/StandardMacros.IsValid` (`self.Newest Tunnel`)
          (:`Is Valid`
            (`self.Spawn Tunnel at Spawn Point`))
          (:`Is Not Valid`
            (`self.SpawnTunnel` (`self.K2_GetActorLocation` (`GameplayStatics.GetPlayerPawn` 0)))))))))

(fn `Spawn Tunnel at Spawn Point`
  (`self.SpawnTunnel` (`SceneComponent.K2_GetComponentLocation` (`/Game/InfiniteMatrix/Blueprints/BP_Tunnel.SpawnPoint` (`self.Newest Tunnel`)))))

(fn `SpawnTunnel`
  (params (SpawnLocation :type "Vector Structure"))
  (bind _returnvalue (+ SpawnLocation (`KismetMathLibrary.MakeVector` 1000.0 (`KismetMathLibrary.RandomFloatInRange` 0.0 200.0) (`KismetMathLibrary.RandomFloatInRange` 0.0 200.0))))
  (bind _returnvalue_2 (`|SpawnActorFromClass` "/Game/InfiniteMatrix/Blueprints/BP_Tunnel.BP_Tunnel_C" (`KismetMathLibrary.MakeTransform` SpawnLocation) "Undefined" "MultiplyWithRoot" null null))
  (bind _output_get (set `self.Newest Tunnel` _returnvalue_2))
  (set `/Game/InfiniteMatrix/Blueprints/BP_Tunnel.Tunnel Spawner` self _output_get)
  (`/Game/InfiniteMatrix/Blueprints/BP_Tunnel.RandomizeWall` _output_get)
  (if (> (`KismetMathLibrary.RandomIntegerInRange` 0 6) 5)
    (`|SpawnActorFromClass` "/Game/InfiniteMatrix/Blueprints/BP_Healthpacks.BP_Healthpacks_C" (`KismetMathLibrary.MakeTransform` _returnvalue) "Undefined" "MultiplyWithRoot" null null)
    (elif (> (`KismetMathLibrary.RandomIntegerInRange` 0 6) 5)
      (`|SpawnActorFromClass` "/Game/InfiniteMatrix/Blueprints/BP_Enemy.BP_Enemy_C" (`KismetMathLibrary.MakeTransform` (+ _returnvalue (1000.0 0.0 0.0))) "Undefined" "MultiplyWithRoot" null null)
      (`KismetSystemLibrary.PrintString` "Enemy"))))

(fn `UserConstructionScript`)